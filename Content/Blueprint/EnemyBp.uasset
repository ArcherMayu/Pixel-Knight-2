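; Paper2D side-view enemy character that patrols, melee-attacks the player and dies when its health runs out.
; Tick drives flipbooks and walking, with a forward line trace that pauses and reverses patrol at obstacles.
; Box overlap with Spritechar runs a looping attack timer; after the attack animation, a short pawn trace damages the player.
; Taking damage launches it in knockback, and death plays a flipbook before destroying the actor.
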(event OnComponentEndOverlap(Box)
  (params (OverlappedComponent :type Primitive%20Component%20Object%20Reference) (OtherActor :type Actor%20Object%20Reference) (OtherComp :type Primitive%20Component%20Object%20Reference) (OtherBodyIndex :type Integer))
  (bind _returnvalue (Transformation|GetActorLocation))
  (Utilities|Casting|CastToSpritechar OtherActor)
  (Utilities|Time|ClearandInvalidateTimerbyHandle (Variables|Default|GetAttack%20Event))
  (Utilities|FlowControl|DoOnce false) ; enters at Reset
)

(event OnComponentBeginOverlap(Box)
  (params (OverlappedComponent :type Primitive%20Component%20Object%20Reference) (OtherActor :type Actor%20Object%20Reference) (OtherComp :type Primitive%20Component%20Object%20Reference) (OtherBodyIndex :type Integer) (bFromSweep :type Boolean) (SweepResult :type Hit%20Result%20Structure%20%28by%20ref%29))
  (Utilities|Casting|CastToSpritechar OtherActor)
  (bind _returnvalue (Utilities|Time|SetTimerbyEvent (delegate Custom|Attack%20Player) 1.0 true))
  (Variables|Default|SetAttack%20Event _returnvalue))

(event Custom|Attack%20Player
  (bind _returnvalue (Transformation|GetActorLocation))
  (if (not (Variables|Default|GetIsdead?))
    (Utilities|FlowControl|DoOnce false :!label _label
      (:Completed
        (Variables|Default|SetIs%20Enemy%20Attacking true)
        (Utilities|FlowControl|Delay (Class|PaperFlipbook|GetTotalDuration (Variables|Default|Getattack)))
        (Utilities|FlowControl|Sequence
          (:then_0
            (Variables|Default|SetIs%20Enemy%20Attacking false))
          (:then_1
            (bind _outhit (Collision|LineTraceForObjects _returnvalue (+ _returnvalue (* (Transformation|GetActorForwardVector) "-90.000000,0.000000,0.000000")) (Utilities|Array|MakeArray "ObjectTypeQuery3") false (Utilities|Array|MakeArray self) "None"))
            (if (== (.HitActor (Collision|BreakHitResult _outhit)) (Game|GetPlayerCharacter 0))
              (Game|Damage|ApplyDamage (.HitActor (Collision|BreakHitResult _outhit)) 1.0 0 self)
              (Utilities|FlowControl|Delay 0.8)
              (goto _label Reset))))))))

(event Custom|Animation%20Update
  (Sprite|SetFlipbook (Variables|Default|GetSprite) (select (> (Math|Vector|VectorLength (Variables|/Script/Engine.MovementComponent|GetVelocity (Variables|Character|GetCharacterMovement))) 0.0) (Variables|Default|Getwalk) (Variables|Default|GetDeathIdle))))

(event Custom|Movement
  (bind _returnvalue (Transformation|GetActorLocation))
  (Utilities|FlowControl|Sequence
    (:then_0
      (if (> (Variables|Default|Getmovdir) 0.0)
        (Transformation|SetActorRotation "0, 0, 0")
        (else
          (Transformation|SetActorRotation "0.000000,180.000000,0.000000"))))
    (:then_1
      (Pawn|Input|AddMovementInput "-1.000000,0.000000,0.000000" (Variables|Default|Getmovdir) false)
      (bind _returnvalue_2 (Collision|LineTraceByChannel _returnvalue (+ _returnvalue (* (Transformation|GetActorForwardVector) (Math|Vector|MakeVector -2e+02 0.0 0.0))) "TraceTypeQuery1" false 0 "None"))
      (if _returnvalue_2
        (Utilities|FlowControl|DoOnce false :!label _label
          (:Completed
            (Variables|/Script/Engine.CharacterMovementComponent|SetMaxWalkSpeed (Variables|Character|GetCharacterMovement) 0.0)
            (Utilities|FlowControl|Delay (Variables|Default|GetDuration))
            (Variables|/Script/Engine.CharacterMovementComponent|SetMaxWalkSpeed (Variables|Character|GetCharacterMovement) (Variables|Default|GetMax%20Walk%20Speed))
            (Variables|Default|Setmovdir (* (Variables|Default|Getmovdir) -1.0))
            (goto _label Reset)))))))

(event EventBeginPlay
  (Variables|/Script/Engine.CharacterMovementComponent|SetMaxWalkSpeed (Variables|Character|GetCharacterMovement) (Variables|Default|GetMax%20Walk%20Speed)))

(event Collision|EventActorBeginOverlap
  (params (OtherActor :type Actor%20Object%20Reference)))

(event EventTick
  (params (DeltaSeconds :type Float%20%28single-precision%29))
  (if (not (Variables|Default|GetIsdead?))
    (if (Variables|Default|GetIs%20Enemy%20Attacking)
      (Sprite|SetFlipbook (Variables|Default|GetSprite) "/Game/PNG/Bringer-Of-Death/Individual_Sprite/Attack/Bringer-of-Death_Attack.Bringer-of-Death_Attack")
      (Utilities|FlowControl|Delay (Class|PaperFlipbook|GetTotalDuration (Variables|Default|Getattack)))
      (Variables|Default|SetIs%20Enemy%20Attacking false)
      (else
        (CallFunction|AnimationUpdate)
        (CallFunction|Movement)))))

(event Game|Damage|EventAnyDamage
  (params (Damage :type Float%20%28single-precision%29) (DamageType :type Damage%20Type%20Object%20Reference) (InstigatedBy :type Controller%20Object%20Reference) (DamageCauser :type Actor%20Object%20Reference))
  (Variables|Default|SetGolem_health (- (Variables|Default|GetGolem_health) Damage))
  (Character|LaunchCharacter (* (select (< (.x (Math|Vector|Normalize (Math|Vector|GetUnitDirection(Vector) (Transformation|GetActorLocation DamageCauser) (Transformation|GetActorLocation)))) 0.0) "1.000000,0.000000,0.000000" "-1.000000,0.000000,0.000000") "-500.000000,0.000000,100.000000") false false)
  (if (<= (Variables|Default|GetGolem_health) 0.0)
    (Variables|Default|SetIsdead? true)
    (Sprite|SetFlipbook (Variables|Default|GetSprite) "/Game/PNG/Bringer-Of-Death/Individual_Sprite/Death/Bringer-of-Death_Death.Bringer-of-Death_Death")
    (Utilities|FlowControl|Delay (Class|PaperFlipbook|GetTotalDuration (Variables|Default|GetDeathDeath)))
    (Actor|DestroyActor)
    (else
      (Variables|Default|SetIsdead? false))))

(fn ConstructionScript)